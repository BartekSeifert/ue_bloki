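; Camera pawn that shows the main UI and lets the player recolor actors under the mouse cursor.
; CameraRight and CameraLeft both yaw the pawn by +90 degrees, and ColorPicker toggles the color picker widget.
; Without an active HMD, Tick caches the hovered actor from a cursor trace.
; With the picker open, left-click creates a dynamic material instance on that actor's primitive component and sets its "Color" parameter from the widget.
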(event `CameraRight`
  ;[1 1 1] CameraRotateRight
  (`self.K2_SetActorRotation` self (`KismetMathLibrary.MakeRotator` (.roll (`self.K2_GetActorRotation` self)) (.pitch (`self.K2_GetActorRotation` self)) (+ (.yaw (`self.K2_GetActorRotation` self)) 90.0)) false))

(event `CameraLeft`
  ;[1 1 1] CameraRotateRight
  (`self.K2_SetActorRotation` self (`KismetMathLibrary.MakeRotator` (.roll (`self.K2_GetActorRotation` self)) (.pitch (`self.K2_GetActorRotation` self)) (+ (.yaw (`self.K2_GetActorRotation` self)) 90.0)) false))

(event `self.ReceiveTick`
  (params (DeltaSeconds :type "Float (single-precision)"))
  (bind (_bblockinghit _binitialoverlap _time _distance _location _impactpoint _normal _impactnormal _physmat _hitactor) (`GameplayStatics.BreakHitResult` (`PlayerController.GetHitResultUnderCursorByChannel` (`GameplayStatics.GetPlayerController` 0) "TraceTypeQuery1" true)))
  ;[1 1 1] Hover Actor
  (if (not (`HeadMountedDisplayFunctionLibrary.IsHeadMountedDisplayEnabled`))
    (`/Engine/EditorBlueprintResources/StandardMacros.IsValid` _hitactor
      (:`Is Valid`
        (set `self.HoverActor` _hitactor)
        (set `self.Phys Mat` _physmat)))))

(event `self.ReceiveBeginPlay`
  ;[1 1 1] show/hide main ui
  (bind _returnvalue (`|CreateWidget` "/Game/UI/BP_UI.BP_UI_C"))
  (bind _output_get (set `self.MainUI` _returnvalue))
  (`UserWidget.AddToViewport` _output_get 0))

(event `ColorPicker`
  (`/Engine/EditorBlueprintResources/StandardMacros.FlipFlop`
    (:`A`
      (bind _returnvalue (`|CreateWidget` "/Game/UI/ColorPickerWidget.ColorPickerWidget_C" null null))
      (`UserWidget.AddToViewport` _returnvalue 0)
      (set `self.ColorOn` true))
    (:`B`
      (bind _foundwidgets (`WidgetBlueprintLibrary.GetAllWidgetsOfClass` "/Game/UI/ColorPickerWidget.ColorPickerWidget_C"))
      (`Widget.RemoveFromParent` (`|GetArrayItem` _foundwidgets))
      (set `self.ColorOn` false))))

(event `Key|LeftMouseButton`
  (params (Key :type "Key Structure"))
  (bind _returnvalue (`self.GetComponentByClass` (`self.HoverActor`) "/Script/Engine.PrimitiveComponent"))
  (bind _returnvalue_2 (`PrimitiveComponent.GetMaterial` _returnvalue 0))
  ;[1 1 1] Create DMI
  (:`Pressed`
    (if (`self.ColorOn`)
      (`/Engine/EditorBlueprintResources/StandardMacros.IsValid` _returnvalue
        (:`Is Valid`
          (`|ExecutionSequence`
            (:`then_0`
              (`PrimitiveComponent.SetMaterial` _returnvalue 0 _returnvalue_2))
            (:`then_1`
              (`KismetSystemLibrary.PrintString` "Hello")
              (bind _returnvalue_3 (`PrimitiveComponent.CreateDynamicMaterialInstance` _returnvalue 0 _returnvalue_2 "None"))
              (`MaterialInstanceDynamic.SetVectorParameterValue` _returnvalue_3 "Color" (`/Game/UI/ColorPickerWidget.Background Color` (stale `ColorPicker` _returnvalue))))))
        (:`Is Not Valid`
          (`KismetSystemLibrary.PrintString` "Is not Valid"))))))

(fn `UserConstructionScript`)