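; Camera controller that drives BP_CameraPawn with axis movement, mouse panning and orthographic zoom, plus pan and zoom resets.
; Movement scales with spring arm length and a Shift multiplier, holds default height when strafing, and must stay inside an optional BP_CameraMovementVolume box.
; Holding Pan opens gates for yaw and clamped pitch rotation while blocking movement; zoom adjusts clamped ortho width.
; Screen-edge scrolling logic exists but is disconnected.
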(event `self.ReceiveBeginPlay`
  (`|ExecutionSequence`
    (:`then_0`
      (`self.ReferenceCasts`))
    (:`then_1`
      (`self.FindCameraMovementVolume`))))

(event `self.ReceiveTick`
  (params (DeltaSeconds :type "Float (single-precision)")))

(event `InputAxis|MoveForward`
  (params (AxisValue :type "Float (single-precision)"))
  (bind _transform (`self.MovementX` (`self.MovementSpeedCalculation`) (`self.FastMoveMultiplayer`) AxisValue (`self.BP_CameraPawnRef`)))
  ;[1 1 1] Movement X
  (if (`self.DisableCamNav`)
    _
    (elif (`self.CheckNewCameraLocation` (.location _transform))
      (`self.K2_SetActorTransform` (`self.BP_CameraPawnRef`) _transform false false))))

(event `InputAxis|MoveRight`
  (params (AxisValue :type "Float (single-precision)"))
  (bind _returnvalue (`KismetMathLibrary.MakeVector` (.x (.location (`self.MovementY` (`self.MovementSpeedCalculation`) (`self.FastMoveMultiplayer`) AxisValue (`self.BP_CameraPawnRef`)))) (.y (.location (`self.MovementY` (`self.MovementSpeedCalculation`) (`self.FastMoveMultiplayer`) AxisValue (`self.BP_CameraPawnRef`)))) (`self.DefaultCameraPawnZLoc`)))
  ;[1 1 1] Movement Y
  (if (`self.DisableCamNav`)
    _
    (elif (`self.CheckNewCameraLocation` _returnvalue)
      (`self.K2_SetActorTransform` (`self.BP_CameraPawnRef`) (`KismetMathLibrary.MakeTransform` _returnvalue (.rotation (`self.MovementY` (`self.MovementSpeedCalculation`) (`self.FastMoveMultiplayer`) AxisValue (`self.BP_CameraPawnRef`))) (.scale (`self.MovementY` (`self.MovementSpeedCalculation`) (`self.FastMoveMultiplayer`) AxisValue (`self.BP_CameraPawnRef`)))) false false))))

(event `InputAction|PanReset`
  (params (Key :type "Key Structure"))
  (bind _bp_camerapawnref (`self.BP_CameraPawnRef`))
  ;[1 1 1] Pan Reset
  (:`Pressed`
    (`self.K2_SetActorRotation` _bp_camerapawnref (`KismetMathLibrary.MakeRotator` (.roll (`self.K2_GetActorRotation` _bp_camerapawnref))) false)))

(event `InputAxisKey|MouseX`
  (params (AxisValue :type "Float (single-precision)"))
  ;[1 1 1] Pan X
  (`/Engine/EditorBlueprintResources/StandardMacros.Gate` true :!label _label
    (:`Exit`
      (`self.K2_SetActorRotation` (`self.BP_CameraPawnRef`) (`KismetMathLibrary.MakeRotator` (.roll (`self.K2_GetActorRotation` (`self.BP_CameraPawnRef`))) (.pitch (`self.K2_GetActorRotation` (`self.BP_CameraPawnRef`))) (+ (.yaw (`self.K2_GetActorRotation` (`self.BP_CameraPawnRef`))) (* (`self.PanSensitivity`) AxisValue))) false))))

(event `InputAction|Pan`
  (params (Key :type "Key Structure"))
  ;[1 1 1] Pan X
  (:`Pressed`
    (set `self.DisableCamNav` true)
    (goto _label :!via `Open`))
  (:`Released`
    (set `self.DisableCamNav` false)
    (goto _label :!via `Close`)))

(event `Key|LeftShift`
  (params (Key :type "Key Structure"))
  ;[1 1 1] Move Multiplayer
  (:`Pressed`
    (set `self.FastMoveMultiplayer` 2.0))
  (:`Released`
    (set `self.FastMoveMultiplayer` 1.0)))

(event `InputAxisKey|MouseY`
  (params (AxisValue :type "Float (single-precision)"))
  ;[1 1 1] Pan Y
  (`/Engine/EditorBlueprintResources/StandardMacros.Gate` true :!label _label_2
    (:`Exit`
      (`self.K2_SetActorRotation` (`self.BP_CameraPawnRef`) (`KismetMathLibrary.MakeRotator` (.roll (`self.K2_GetActorRotation` (`self.BP_CameraPawnRef`))) (`KismetMathLibrary.FClamp` (+ (.pitch (`self.K2_GetActorRotation` (`self.BP_CameraPawnRef`))) (* (`self.PanSensitivity`) AxisValue)) -15.0 45.0) (.yaw (`self.K2_GetActorRotation` (`self.BP_CameraPawnRef`)))) false))))

(event `InputAction|Pan`
  (params (Key :type "Key Structure"))
  ;[1 1 1] Pan Y
  (:`Pressed`
    (set `self.DisableCamNav` true)
    (goto _label_2 :!via `Open`))
  (:`Released`
    (set `self.DisableCamNav` false)
    (goto _label_2 :!via `Close`)))

(event `InputAction|ZoomIn`
  (params (Key :type "Key Structure"))
  (bind _camera (`/Game/BLOKI/Blueprints/MyGame/BP_CameraPawn.Camera` (`self.BP_CameraPawnRef`)))
  ;[1 1 1] Zoom IN/OUT
  (:`Pressed`
    (`CameraComponent.SetOrthoWidth` _camera (`KismetMathLibrary.FClamp` (- (`CameraComponent.OrthoWidth` _camera) (`self.ZoomSensitivity`)) 1024.0 (`self.MaxArmDistance`)))))

(event `InputAxisKey|MouseX`
  (params (AxisValue :type "Float (single-precision)"))
  ;[1 1 1] Edge Movement
)

(event `InputAxisKey|MouseY`
  (params (AxisValue :type "Float (single-precision)"))
  ;[1 1 1] Edge Movement
)

(event `InputAction|ZoomOut`
  (params (Key :type "Key Structure"))
  (bind _camera (`/Game/BLOKI/Blueprints/MyGame/BP_CameraPawn.Camera` (`self.BP_CameraPawnRef`)))
  ;[1 1 1] Zoom IN/OUT
  (:`Pressed`
    (`CameraComponent.SetOrthoWidth` _camera (`KismetMathLibrary.FClamp` (+ (`self.ZoomSensitivity`) (`CameraComponent.OrthoWidth` _camera)) 1024.0 (`self.MaxArmDistance`)))))

(event `InputAction|ZoomReset`
  (params (Key :type "Key Structure"))
  ;[1 1 1] ZoomReset
  (:`Pressed`
    (`CameraComponent.SetOrthoWidth` (`/Game/BLOKI/Blueprints/MyGame/BP_CameraPawn.Camera` (`self.BP_CameraPawnRef`)) (`self.DefaultCameraOrtoWidth`))))

(fn `CheckNewCameraLocation`
  (params (NewCameraLocation :type "Vector Structure"))
  (returns (IsInMovementVolume :type Boolean))
  (bind _cameramovementvolume (`self.CameraMovementVolume`)
    (:`then`
      (bind _box (`/Game/BLOKI/Blueprints/MyGame/BP_CameraMovementVolume.Box` _cameramovementvolume))
      (return (`KismetMathLibrary.IsPointInBoxWithTransform` NewCameraLocation (`SceneComponent.K2_GetComponentToWorld` _box) (`BoxComponent.BoxExtent` _box))))
    (:`else`
      (return true))))

(fn `FindCameraMovementVolume`
  (bind _returnvalue (`GameplayStatics.GetActorOfClass` "/Game/BLOKI/Blueprints/MyGame/BP_CameraMovementVolume.BP_CameraMovementVolume_C"))
  (set `self.CameraMovementVolume` _returnvalue))

(fn `MovementSpeedCalculation`
  (returns (MoveSensitivity :type "Float (double-precision)"))
  (return (`KismetMathLibrary.FClamp` (/ (`SpringArmComponent.TargetArmLength` (`/Game/BLOKI/Blueprints/MyGame/BP_CameraPawn.SpringArm` (`self.BP_CameraPawnRef`))) 100.0) 5.0 20.0)))

(fn `UserConstructionScript`)