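; Camera pawn for a building customization tool that adds the main tools widget at start and yaws in 90-degree steps, with both left and right events turning +90.
; Outside VR, left click traces under the cursor and acts by the current edit mode.
; Color and balcony modes send change messages to the hit actor.
; Greenery (Zielen) mode spawns a terrain object on BP_ground components when a box overlap finds the spot free.
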(event `CameraRight`
  ;[1 1 1] CameraRotateRight
  (`self.K2_SetActorRotation` self (`KismetMathLibrary.MakeRotator` (.roll (`self.K2_GetActorRotation` self)) (.pitch (`self.K2_GetActorRotation` self)) (+ (.yaw (`self.K2_GetActorRotation` self)) 90.0)) false))

(event `CameraLeft`
  ;[1 1 1] CameraRotateRight
  (`self.K2_SetActorRotation` self (`KismetMathLibrary.MakeRotator` (.roll (`self.K2_GetActorRotation` self)) (.pitch (`self.K2_GetActorRotation` self)) (+ (.yaw (`self.K2_GetActorRotation` self)) 90.0)) false))

(event `Key|LeftMouseButton`
  (params (Key :type "Key Structure"))
  (bind (_bblockinghit _binitialoverlap _time _distance _location _impactpoint _normal _impactnormal _physmat _hitactor _hitcomponent) (`GameplayStatics.BreakHitResult` (`PlayerController.GetHitResultUnderCursorByChannel` (`GameplayStatics.GetPlayerController` 0) "TraceTypeQuery1" true)))
  (:`Pressed`
    ;[1 1 1] Hover Actor
    (if (not (`HeadMountedDisplayFunctionLibrary.IsHeadMountedDisplayEnabled`))
      (`/Engine/EditorBlueprintResources/StandardMacros.IsValid` _hitactor
        (:`Is Valid`
          (switch `/Game/BLOKI/Blueprints/MyGame/EEditionMode` (`self.CurrentEdytionMode`)
            (:`NewEnumerator0`
              (message `/Game/BLOKI/Blueprints/Interfaces/BPI_Interaction.ChangeBaseColor` _hitactor _hitcomponent (`self.BaseColor`) (`self.Wzor`)))
            (:`NewEnumerator1`
              (message `/Game/BLOKI/Blueprints/Interfaces/BPI_Interaction.ChangeAccentColor` _hitactor _hitcomponent (`self.AccentColor`) (`self.Wzor`)))
            (:`NewEnumerator2`
              (message `/Game/BLOKI/Blueprints/Interfaces/BPI_Interaction.ChangeBalconyType` _hitactor _hitcomponent (`self.BalconyMesh`)))
            (:`NewEnumerator4`
              (cast `/Game/BLOKI/Geometry/BP_ground` _hitactor)
              (`self.Create Terrain Object` _hitcomponent (`self.ZielenMesh`)))))))))

(event `self.ReceiveBeginPlay`
  ;[1 1 1] show/hide main ui
  (bind _returnvalue (`|CreateWidget` "/Game/BLOKI/UI/ToolsWidget.ToolsWidget_C"))
  (bind _output_get (set `self.MainUI` _returnvalue))
  (`UserWidget.AddToViewport` _output_get 0))

(event `ChangeEditionMode`
  (params (EditionMode :type "/Game/BLOKI/Blueprints/MyGame/EEditionMode Enum" :default "NewEnumerator3"))
  ;[1 1 1] Change Edition Mode
  (set `self.CurrentEdytionMode` EditionMode))

(event `Create Terrain Object`
  (params (PrimitiveComponent :type "PrimitiveComponent Object Reference") (StaticMesh :type "StaticMesh Object Reference"))
  (bind (_returnvalue_origin _returnvalue_boxextent) (`KismetMathLibrary.BreakBoxSphereBounds` (`StaticMesh.GetBounds` StaticMesh)))
  (bind _returnvalue_location (`KismetMathLibrary.BreakTransform` (`SceneComponent.K2_GetComponentToWorld` PrimitiveComponent)))
  (bind (_outactors _returnvalue) (`KismetSystemLibrary.BoxOverlapActors` _returnvalue_location _returnvalue_boxextent (`|MakeArray` "ObjectTypeQuery7" :!type "EObjectTypeQuery Enum")))
  (if (not _returnvalue)
    (`|SpawnActorFromClass` "/Game/BLOKI/Blueprints/MyGame/BP_TerrainObject.BP_TerrainObject_C" (`KismetMathLibrary.MakeTransform` _returnvalue_location (struct :`Yaw` -30.0)) "AlwaysSpawn" "OverrideRootScale" null (`self.ZielenMesh`) null)))

(fn `UserConstructionScript`)