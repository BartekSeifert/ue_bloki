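; BP_big_block is a big building block actor whose colors, patterns and balcony meshes can be changed through events.
; Base and accent color events each create a dynamic material instance on the given component and set its Color and Wzor texture parameters.
; The balcony event swaps a static mesh only after a check on the component's parents, then picks the flower or left balcony material according to the mesh.
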(event `/Game/BLOKI/Blueprints/Interfaces/BPI_Interaction.ChangeBaseColor`
  (params (Component :type "PrimitiveComponent Object Reference") (Color :type "LinearColor Structure") (Texture :type "Texture2D Object Reference"))
  (bind _returnvalue (`PrimitiveComponent.CreateDynamicMaterialInstance` Component 0 (`PrimitiveComponent.GetMaterial` Component 0) "None"))
  (`MaterialInstanceDynamic.SetVectorParameterValue` _returnvalue "Color" Color)
  (`MaterialInstanceDynamic.SetTextureParameterValue` _returnvalue "Wzor" Texture))

(event `/Game/BLOKI/Blueprints/Interfaces/BPI_Interaction.ChangeAccentColor`
  (params (Component :type "PrimitiveComponent Object Reference") (Color :type "LinearColor Structure") (Texture :type "Texture2D Object Reference"))
  (bind _returnvalue (`PrimitiveComponent.CreateDynamicMaterialInstance` Component 0 (`PrimitiveComponent.GetMaterial` Component 0) "None"))
  (`MaterialInstanceDynamic.SetVectorParameterValue` _returnvalue "Color" Color)
  (`MaterialInstanceDynamic.SetTextureParameterValue` _returnvalue "Wzor" Texture))

(event `/Game/BLOKI/Blueprints/Interfaces/BPI_Interaction.ChangeBalconyType`
  (params (Component :type "PrimitiveComponent Object Reference") (BalconyMesh :type "StaticMesh Object Reference"))
  (bind _asstatic_mesh_component (cast `StaticMeshComponent` Component))
  (bind _parents (`SceneComponent.GetParentComponents` _asstatic_mesh_component))
  (if (or (>= (`KismetArrayLibrary.Array_Find` _parents) 0) (>= (`KismetArrayLibrary.Array_Find` _parents) 0))
    (`StaticMeshComponent.SetStaticMesh` _asstatic_mesh_component BalconyMesh)
    (if (== BalconyMesh "/Game/BLOKI/Geometry/Balkony/b_kwiaty/Geometries/b_kwiaty.b_kwiaty")
      (`PrimitiveComponent.SetMaterial` _asstatic_mesh_component 0 "/Game/BLOKI/Material/Mi_BALKON_KWIATY.Mi_BALKON_KWIATY")
      (else
        (`PrimitiveComponent.SetMaterial` _asstatic_mesh_component 0 "/Game/BLOKI/Material/Mi_BALKON_LEWY.Mi_BALKON_LEWY")))))

(fn `UserConstructionScript`)